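; ItemBase is a base item actor that sits on a ShelfBase parent actor and can be picked up.
; On BeginPlay it casts its parent actor to ShelfBase and caches its own transform relative to that shelf.
; Every Tick recomposes that offset with the shelf's transform and teleports the static mesh there.
; PickedUp detaches the actor and sets Held, but Tick never checks that flag, so the mesh keeps following the shelf.
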(event `self.ReceiveBeginPlay`
  (`self.Initialize`))

(event `self.ReceiveTick`
  (params (DeltaSeconds :type "Float (single-precision)"))
  (`self.UpdateItemLocation` DeltaSeconds))

(event `PickedUp`
  (`self.DetachFromShelf`))

(fn `DetachFromShelf`
  (`self.K2_DetachFromActor` "KeepWorld" "KeepWorld" "KeepWorld")
  (set `self.Held` true))

(fn `Initialize`
  (bind _asshelf_base (cast `/Game/Blueprints/ShelfBase` (`self.GetParentActor`)))
  (bind _output_get (set `self.OwningShelf` _asshelf_base))
  (set `self.InitialTransform` (`KismetMathLibrary.ComposeTransforms` (`self.GetTransform`) (`KismetMathLibrary.InvertTransform` (`self.GetTransform` _output_get)))))

(fn `UpdateItemLocation`
  (params (DeltaTime :type "Float (double-precision)"))
  (`SceneComponent.K2_SetWorldTransform` (`self.StaticMesh`) (`KismetMathLibrary.ComposeTransforms` (`self.InitialTransform`) (`self.GetTransform` (`self.OwningShelf`))) false true))

(fn `UserConstructionScript`)