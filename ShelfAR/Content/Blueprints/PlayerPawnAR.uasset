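; AR player pawn that turns touch input into shelf placement, shelf moving and item picking, based on the current interact mode.
; A touch spawns a test shelf on traced AR geometry, then switches to move mode, where touches drag shelves until release.
; Deprojected screen traces on separate channels select shelves or items.
; The lock button enables picking, and a pick switches to rotate mode, which has no touch handling here.
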(event `InputTouch`
  (params (Location :type "Vector Structure") (FingerIndex :type "ETouchIndex Enum"))
  (bind _screencoords (`self.ScreenCoordsFromTouch` FingerIndex))
  (:`Pressed`
    (`self.InitializeTouchLocation` FingerIndex)
    (switch `/Game/Blueprints/PawnInteractionMode` (`self.CurrentInteractMode`)
      (:`NewEnumerator0`
        (`self.SpawnShelf` _screencoords))
      (:`NewEnumerator1`
        (`self.SelectShelfForMoving` _screencoords))
      (:`NewEnumerator2`
        (`self.SelectItem` _screencoords))))
  (:`Released`
    (`self.FinishMovingShelf`))
  (:`Moved`
    (switch `/Game/Blueprints/PawnInteractionMode` (`self.CurrentInteractMode`)
      (:`NewEnumerator1`
        (`self.MoveShelf` _screencoords)))))

(event `LockButtonPressed`
  (set `self.CurrentInteractMode` "NewEnumerator2"))

(fn `FinishMovingShelf`
  (bind _movedshelf (`self.MovedShelf`))
  (`/Engine/EditorBlueprintResources/StandardMacros.IsValid` _movedshelf
    (:`Is Valid`
      (`/Game/Blueprints/ShelfBase.EndMove` _movedshelf)
      (set `self.MovedShelf` null))))

(fn `InitializeTouchLocation`
  (params (Index :type "ETouchIndex Enum" :default "Touch1"))
  (`KismetArrayLibrary.Array_Set` (`self.PreviousTouchLocation`) (`KismetMathLibrary.Conv_ByteToInt` Index) (`self.ScreenCoordsFromTouch` Index)))

(fn `MoveShelf`
  (params (NewScreenCoords :type "Vector2D Structure"))
  (bind _movedshelf (`self.MovedShelf`))
  (`/Engine/EditorBlueprintResources/StandardMacros.IsValid` _movedshelf
    (:`Is Valid`
      (`/Game/Blueprints/ShelfBase.Move` _movedshelf NewScreenCoords))))

(fn `ScreenCoordsFromTouch`
  (params (TouchIndex :type "ETouchIndex Enum" :default "Touch1"))
  (returns (ScreenCoords :type "Vector2D Structure"))
  (bind (_locationx _locationy) (`PlayerController.GetInputTouchState` (`GameplayStatics.GetPlayerController` 0) TouchIndex))
  (return (`KismetMathLibrary.MakeVector2D` _locationx _locationy)))

(fn `ScreenTrace`
  (params (ScreenCoords :type "Vector2D Structure") (TraceChannel :type "ETraceTypeQuery Enum" :default "TraceTypeQuery1"))
  (returns (`Hit Actor` :type "Actor Object Reference"))
  (bind (_worldposition _worlddirection) (`GameplayStatics.DeprojectScreenToWorld` (`GameplayStatics.GetPlayerController` 0) ScreenCoords))
  (bind _outhits (`KismetSystemLibrary.LineTraceMulti` _worldposition (+ _worldposition (* _worlddirection 999999.0)) TraceChannel))
  (bind (_output_bblockinghit _output_binitialoverlap _output_time _output_distance _output_location _output_impactpoint _output_normal _output_impactnormal _output_physmat _output_hitactor) (`GameplayStatics.BreakHitResult` (`|GetArrayItem` _outhits)))
  (return _output_hitactor))

(fn `SelectItem`
  (params (ScreenCoords :type "Vector2D Structure"))
  (bind _hit_actor (`self.ScreenTrace` ScreenCoords "TraceTypeQuery4"))
  (bind _asitem_base (cast `/Game/Blueprints/ItemBase` _hit_actor))
  (bind _output_get (set `self.PickedItem` _asitem_base))
  (`/Game/Blueprints/ItemBase.PickedUp` _output_get)
  (set `self.CurrentInteractMode` "NewEnumerator3"))

(fn `SelectShelfForMoving`
  (params (ScreenCoords :type "Vector2D Structure"))
  (bind _hit_actor (`self.ScreenTrace` ScreenCoords "TraceTypeQuery3"))
  (bind _asshelf_base (cast `/Game/Blueprints/ShelfBase` _hit_actor))
  (bind _output_get (set `self.MovedShelf` _asshelf_base))
  (`/Game/Blueprints/ShelfBase.BeginMove` _output_get ScreenCoords))

(fn `SpawnShelf`
  (params (ScreenCoord :type "Vector2D Structure"))
  (bind _returnvalue (`ARBlueprintLibrary.LineTraceTrackedObjects` ScreenCoord false false false))
  (if (> (`KismetArrayLibrary.Array_Length` _returnvalue) 0)
    (bind _output (`|GetArrayItem` _returnvalue))
    (`|SpawnActorFromClass` "/Game/Blueprints/Shelves/TestShelf.TestShelf_C" (`ARTraceResultLibrary.GetLocalToWorldTransform` _output) "AlwaysSpawn" "OverrideRootScale" null (`ARTraceResultLibrary.GetTrackedGeometry` _output) null)
    (set `self.CurrentInteractMode` "NewEnumerator1")))

(fn `UserConstructionScript`)