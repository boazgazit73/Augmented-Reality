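; Base shelf actor for AR that stays pinned to tracked geometry and can be moved across that surface through screen-space input.
; It pins its static mesh on BeginPlay and EndMove, and unpins it on BeginMove.
; BeginMove stores the screen offset between actor and input point, so the shelf keeps its grab point.
; Move deprojects the offset position and intersects that ray with the geometry's infinite plane to place the actor.
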(event `self.ReceiveBeginPlay`
  (`self.LockToSurface`))

(event `self.ReceiveTick`
  (params (DeltaSeconds :type "Float (single-precision)")))

(event `BeginMove`
  (params (InitialScreenCoords :type "Vector2D Structure"))
  (`ARBlueprintLibrary.UnpinComponent` (`self.StaticMesh`))
  (`self.CalculateMoveOffset` InitialScreenCoords))

(event `Move`
  (params (NewScreenCoords :type "Vector2D Structure"))
  (`self.MoveShelf` NewScreenCoords))

(event `EndMove`
  (`self.LockToSurface`))

(fn `CalculateMoveOffset`
  (params (ScreenCoords :type "Vector2D Structure"))
  (set `self.MoveOffset` (- (`GameplayStatics.ProjectWorldToScreen` (`GameplayStatics.GetPlayerController` 0) (`self.K2_GetActorLocation`)) ScreenCoords)))

(fn `LockToSurface`
  (`ARBlueprintLibrary.PinComponent` (`self.StaticMesh`) (`SceneComponent.K2_GetComponentToWorld` (`self.StaticMesh`)) (`self.TrackedGeometry`)))

(fn `MoveShelf`
  (params (ScreenPosition :type "Vector2D Structure (by ref)"))
  (bind (_returnvalue_location _returnvalue_rotation) (`KismetMathLibrary.BreakTransform` (`ARTrackedGeometry.GetLocalToWorldTransform` (`self.TrackedGeometry`))))
  (bind (_worldposition _worlddirection) (`GameplayStatics.DeprojectScreenToWorld` (`GameplayStatics.GetPlayerController` 0) (+ ScreenPosition (`self.MoveOffset`))))
  (bind (_t _intersection _returnvalue) (`KismetMathLibrary.LinePlaneIntersection` _worldposition (+ _worldposition (* _worlddirection 10000.0)) (`KismetMathLibrary.MakePlaneFromPointAndNormal` _returnvalue_location (`KismetMathLibrary.GetUpVector` _returnvalue_rotation))))
  (if _returnvalue
    (`self.K2_SetActorLocation` _intersection)))

(fn `UserConstructionScript`)